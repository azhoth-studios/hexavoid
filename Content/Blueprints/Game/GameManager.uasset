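; GameManager runs the stage and wave loop, creating the stage-end and shop widgets and crossfading music between combat and waiting.
; Each stage derives its wave count and per-wave enemy count from the stage number, then spawns random enemies above shuffled spawnable tiles that are not down.
; Enemies reported through CheckEnd leave the tracked list; an empty list advances the wave or shows the stage-end screen.
; RepairAll repairs every BP_Tile.
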(event `self.ReceiveBeginPlay`
  (bind _returnvalue (`GameplayStatics.GetPlayerController` 0))
  (bind _returnvalue_2 (`|CreateWidget` "/Game/Blueprints/UMG/WBP_StageEnd.WBP_StageEnd_C" _returnvalue self))
  (set `self.StageEndWidget` _returnvalue_2)
  (bind _returnvalue_3 (`|CreateWidget` "/Game/Blueprints/UMG/WBP_Shop.WBP_Shop_C" _returnvalue self))
  (set `self.ShopWidget` _returnvalue_3)
  (bind _returnvalue_4 (`GameplayStatics.GetActorOfClass` "/Game/Blueprints/Character/BP_Character.BP_Character_C"))
  (set `self.Character` _returnvalue_4)
  (`self.StartStage`)
  (bind _returnvalue_5 (`GameplayStatics.SpawnSound2D` "/Game/Sound/GameMusic/kf018905-get-ready-now.kf018905-get-ready-now" 1.0 1.0 0.0 null false false))
  (set `self.Sound` _returnvalue_5))

(event `StartStage`
  (bind _sound (`self.Sound`))
  (bind _fadetime (`self.FadeTime`))
  (bind _stagedelay (`self.StageDelay`))
  (`/Engine/EditorBlueprintResources/StandardMacros.IncrementInt` (`self.Stage`)
    (:`  `
      (`self.StageStart` _stagedelay)
      (`KismetSystemLibrary.Delay` (`KismetMathLibrary.Conv_IntToDouble` _stagedelay))
      (`self.SetWaveCount`
        (:`Completed`
          (`self.StartWave`)
          (`KismetSystemLibrary.Delay` _fadetime)
          (`AudioComponent.SetSound` _sound (`self.StageSound`))
          (`AudioComponent.FadeIn` _sound _fadetime 1.0 0.0 "Linear"))))))

(event `StartWave`
  (bind _tiles (`self.Tiles`))
  (bind _enemycount (`self.EnemyCount`))
  (`self.CalculateWave`
    (:`Completed`
      (`KismetArrayLibrary.Array_Shuffle` _tiles)
      (for _array_element _tiles :!label _label
        (bind _returnvalue (`self.GetTransform` _array_element))
        (bind _returnvalue_2 (`|SpawnActorFromClass` (`KismetArrayLibrary.Array_Random` (`self.TAvailableEnemies`)) (`KismetMathLibrary.MakeTransform` (`KismetMathLibrary.MakeVector` (.x (.location _returnvalue)) (.y (.location _returnvalue)) (+ (.z (.location _returnvalue)) 150.0)) (.rotation _returnvalue) (.scale _returnvalue)) "AdjustIfPossibleButAlwaysSpawn" "OverrideRootScale" null null))
        (set `/Game/Blueprints/Enemy/BP_BaseEnemy.GameManager` self _returnvalue_2)
        (`KismetArrayLibrary.Array_Add` (`self.Enemies`) _returnvalue_2)
        (`/Engine/EditorBlueprintResources/StandardMacros.DecrementInt` _enemycount
          (:`  `
            (if (== _enemycount 0)
              (`self.StopSpawning`))))))))

(event `StopSpawning`
  (goto _label :!via `Break`))

(event `CheckEnd`
  (params (Enemy :type "/Game/Blueprints/Enemy/BP_BaseEnemy Object Reference"))
  (bind _enemies (`self.Enemies`))
  (`KismetArrayLibrary.Array_RemoveItem` _enemies Enemy)
  (if (<= (`KismetArrayLibrary.Array_Length` _enemies) 0)
    (`self.EndWave`)))

(event `EndWave`
  (bind _result (`/Engine/EditorBlueprintResources/StandardMacros.DecrementInt` (`self.Wave`))
    (:`  `
      (if (> _result 0)
        (`self.StartWave`)
        (else
          (`self.EndStage`))))))

(event `EndStage`
  (bind _sound (`self.Sound`))
  (bind _fadetime (`self.FadeTime`))
  ;[1 1 1] Shop
  (`KismetSystemLibrary.Delay` 2.0)
  (`UserWidget.AddToViewport` (`self.StageEndWidget`) 0)
  ;[1 1 1] Start waiting sound
  (`AudioComponent.FadeOut` _sound _fadetime 0.0 "Linear")
  (`KismetSystemLibrary.Delay` _fadetime)
  (`AudioComponent.SetSound` _sound (`self.WaitingSound`))
  (`AudioComponent.FadeIn` _sound _fadetime 1.0 0.0 "Linear"))

(event `RepairAll`
  ;[1 1 1] Repair all
  (bind _outactors (`GameplayStatics.GetAllActorsOfClass` "/Game/Blueprints/Tile/BP_Tile.BP_Tile_C"))
  (for _array_element _outactors
    (`/Game/Blueprints/Tile/BP_Tile.Repair` _array_element)))

(fn `UserConstructionScript`)