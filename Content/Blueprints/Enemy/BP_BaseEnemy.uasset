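; Base enemy character with modular armour meshes that follow the body's pose and a weapon held as a child actor.
; BeginPlay copies fire distance and shot interval into the AI Blackboard and takes ownership of the weapon; Fire shoots slightly below the Blackboard Target character's location.
; Death notifies GameManager before destroying the actor.
; Capsule overlap with a TriggerBox stops the AI brain and prints a debug string.
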(event `self.ReceiveBeginPlay`
  (bind _returnvalue (`AIBlueprintHelperLibrary.GetBlackboard` null))
  (bind _asbp_base_weapon (cast `/Game/Weapon/BP_BaseWeapon` (`ChildActorComponent.ChildActor` (`self.ChildActor`)) :!pure true))
  (`BlackboardComponent.SetValueAsFloat` _returnvalue "FireDistance" (`self.FireDistance`))
  (`BlackboardComponent.SetValueAsFloat` _returnvalue "TimeBetweenShots" (`self.TimeBetweenShots`))
  (set `self.Weapon` _asbp_base_weapon)
  (`self.SetOwner` _asbp_base_weapon self))

(event `OnDeath`
  (`/Game/Blueprints/Game/GameManager.CheckEnd` (`self.GameManager`) self)
  (`self.K2_DestroyActor`))

(event `self.CapsuleComponent.OnComponentBeginOverlap`
  (params (OverlappedComponent :type "PrimitiveComponent Object Reference") (OtherActor :type "Actor Object Reference") (OtherComp :type "PrimitiveComponent Object Reference") (OtherBodyIndex :type Integer) (bFromSweep :type Boolean) (SweepResult :type "HitResult Structure (by ref)"))
  (cast `TriggerBox` OtherActor)
  (`KismetSystemLibrary.PrintString` "Hello")
  (`BrainComponent.StopLogic` (`AIController.BrainComponent` (`AIBlueprintHelperLibrary.GetAIController` self)) ""))

(fn `Fire`
  (`/Game/Weapon/BP_BaseWeapon.Fire` (`self.Weapon`) (- (`self.K2_GetActorLocation` (cast `/Game/Blueprints/Character/BP_Character` (`BlackboardComponent.GetValueAsObject` (`AIBlueprintHelperLibrary.GetBlackboard` null) "Target") :!pure true)) (0.0 0.0 80.0))))

(fn `UserConstructionScript`
  (`SkinnedMeshComponent.SetLeaderPoseComponent` (`self.Helmet`) (`self.Mesh`) false)
  (`SkinnedMeshComponent.SetLeaderPoseComponent` (`self.Chest`) (`self.Mesh`) false)
  (`SkinnedMeshComponent.SetLeaderPoseComponent` (`self.Legs`) (`self.Mesh`) false)
  (`SkinnedMeshComponent.SetLeaderPoseComponent` (`self.Hands`) (`self.Mesh`) false))