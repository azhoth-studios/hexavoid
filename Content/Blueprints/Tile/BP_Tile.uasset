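; BP_Tile is a floor tile that takes two hits to drop away and can be repaired.
; The first hit flags damage through a dynamic material parameter; the second sinks the mesh, then hides it and lets pawns pass through.
; Repair clears damage on a standing tile, or raises a fallen one with visibility and collision restored, polling with a short delay until any fall completes.
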(event `self.ReceiveBeginPlay`
  (bind _returnvalue (`PrimitiveComponent.CreateDynamicMaterialInstance` (`self.StaticMesh`) 0 "/Game/Blueprints/Tile/M_Tile.M_Tile" "None"))
  (set `self.Material` _returnvalue))

(event `OnHit`
  (if (`self.IsHit`)
    (`self.SecondHit`)
    (else
      (`self.FirstHit`))))

(event `FirstHit`
  (set `self.IsHit` true)
  (`MaterialInstanceDynamic.SetScalarParameterValue` (`self.Material`) "Hit" 1.0))

(event `SecondHit`
  (bind _staticmesh (`self.StaticMesh`))
  (if (not (`self.IsDown`))
    (set `self.IsDown` true)
    (`KismetSystemLibrary.MoveComponentTo` _staticmesh (0.0 0.0 -1500.0) (struct) false true 3.0)
    (`SceneComponent.SetVisibility` _staticmesh false false)
    (`PrimitiveComponent.SetCollisionResponseToChannel` (`self.StaticMesh`) "ECC_Pawn" "ECR_Ignore")
    (set `self.IsDownCompleted` true)
    (`MaterialInstanceDynamic.SetScalarParameterValue` (`self.Material`) "Hit" 0.0)))

(event `Repair`
  (bind _staticmesh (`self.StaticMesh`))
  (if (`self.IsDown`)
    (if (`self.IsDownCompleted`) :!label _label
      (`SceneComponent.SetVisibility` _staticmesh true false)
      (`PrimitiveComponent.SetCollisionResponseToChannel` (`self.StaticMesh`) "ECC_Pawn" "ECR_Block")
      (`KismetSystemLibrary.MoveComponentTo` _staticmesh (0.0 0.0 0.0) (struct) true false 1.5)
      (set `self.IsDown` false)
      (set `self.IsDownCompleted` false)
      (set `self.IsHit` false)
      (else
        (`KismetSystemLibrary.Delay` 0.2)
        (goto _label)))
    (else
      (set `self.IsHit` false)
      (`MaterialInstanceDynamic.SetScalarParameterValue` (`self.Material`) "Hit" 0.0))))

(fn `UserConstructionScript`)